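; Player slime pawn for slingshot-style movement in the XZ plane, driven by the IA_Stretch Enhanced Input action.
; Dragging stretches and offsets the physics box; release launches it with impulse and conditional spin, under added downward force.
; A gated Tick interpolates the box back to BaseSize, while mesh and light follow its extent.
; UpdateSize adjusts base size and stretch limit, spawning BP_SlimeDrop on shrinking above the minimum.
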(event OnComponentHit(Box)
  (params (HitComponent :type Primitive%20Component%20Object%20Reference) (OtherActor :type Actor%20Object%20Reference) (OtherComp :type Primitive%20Component%20Object%20Reference) (NormalImpulse :type Vector :default "0, 0, 0") (Hit :type Hit%20Result%20Structure%20%28by%20ref%29))
  (Utilities|Casting|CastToBP_Obstacle_Base OtherActor)
  (Variables|Default|SetInputEnabled false)
  (Variables|Default|SetHitCooldown false)
  (Utilities|FlowControl|Delay 0.5)
  (Variables|Default|SetHitCooldown true))

(event Custom|StopShrinking
  (Utilities|FlowControl|Gate true) ; enters at Close
)

(event Custom|StartShrinking
  (Utilities|FlowControl|Gate true) ; enters at Open
)

(event Input|EnhancedActionEvents|EnhancedInputActionIA_Stretch
  (params (ActionValue :type Vector%202D%20Structure) (ElapsedSeconds :type Float%20%28double-precision%29) (TriggeredSeconds :type Float%20%28double-precision%29) (InputAction :type Input%20Action%20Object%20Reference :default "/Game/BP/Input/IA_Stretch.IA_Stretch"))
  (:Triggered
    (bind _output_get (Variables|Default|SetTouchMoved (Class|KismetMathLibrary|Vector2DInterpto (Variables|Default|GetTouchMoved) ActionValue (Variables|Default|GetDeltaSeconds) 5.0)))
    (CallFunction|CalculateStretchParameters _output_get)
    (CallFunction|UpdateDebugWidget)
    (CallFunction|StretchSlime))
  (:Started
    (bind _output_get_2 (Variables|Default|SetTouchStart ActionValue))
    (Variables|Default|SetTouchMoved _output_get_2)
    (CallFunction|InitDebugWidget)
    (Variables|Default|SetStretchStartLocation (Transformation|GetActorLocation))
    (Class|PrimitiveComponent|SetAngularDamping (Variables|Default|GetBox) 1e+02))
  (:Canceled
    (CallFunction|RemoveDebugWidget :!label _label)
    (CallFunction|StartShrinking))
  (:Completed
    (CallFunction|StretchImpulse)
    (goto _label)))

(event EventBeginPlay
  (Utilities|FlowControl|Sequence
    (:then_0
      (CallFunction|AddMappingInput))))

(event EventTick
  (params (DeltaSeconds :type Float%20%28single-precision%29))
  (bind _box (Variables|Default|GetBox))
  (bind _boxextent (Variables|/Script/Engine.BoxComponent|GetBoxExtent _box))
  (bind _returnvalue (Math|Vector|VectorGetAbs _boxextent))
  (Variables|Default|SetDeltaSeconds DeltaSeconds)
  (Utilities|FlowControl|Sequence
    (:then_0
      (if (Utilities|Operators|NotEqual(!=) (Variables|Default|GetBaseSize) _returnvalue 0.1)
        (Transformation|SetRelativeScale3D (Variables|Default|GetNGS_Slime) (/ _returnvalue 5e+01))
        (Class|RectLightComponent|SetSourceHeight (Variables|Default|GetRectLight) (* (.X (Math|Vector|BreakVector _returnvalue)) 2.0))))
    (:then_1
      (CallFunction|FakeGravity))
    (:then_2
      (Utilities|FlowControl|Gate true
        (:Exit
          (Components|Box|SetBoxExtent (Variables|Default|GetBox) (Math|Interpolation|VInterpTo (Variables|/Script/Engine.BoxComponent|GetBoxExtent (Variables|Default|GetBox)) (Variables|Default|GetBaseSize) (Variables|Default|GetDeltaSeconds) (Variables|Default|GetShrinkingSpeed)) true)
          (if (Utilities|Operators|EqualEqual (Variables|/Script/Engine.BoxComponent|GetBoxExtent (Variables|Default|GetBox)) (Variables|Default|GetBaseSize) 1.0)
            (CallFunction|StopShrinking)))))
    (:then_3
      (if (not (Variables|Default|GetInputEnabled))
        (if (and (<= (Math|Vector|VectorLength (Transformation|GetVelocity)) 25.0) (Variables|Default|GetHitCooldown))
          (Variables|Default|SetInputEnabled true))))))

(event Input|KeyboardEvents|T
  (params (Key :type Key%20Structure :default "None"))
  (:Pressed
    (bind _asplayer_controller (Utilities|Casting|CastToPlayerController (Pawn|GetController)))
    (Class|EnhancedInputSubsystemInterface|InjectInputVectorforAction (PlayerController|LocalPlayerSubsystems|GetEnhancedInputLocalPlayerSubsystem _asplayer_controller) "/Game/BP/Input/IA_Stretch.IA_Stretch" "1.000000,1.000000,0.000000")))

(event Input|KeyboardEvents|R
  (params (Key :type Key%20Structure :default "None"))
  (:Pressed
    (Utilities|FlowControl|FlipFlop
      (:A
        (Game|SetGamePaused true))
      (:B
        (Game|SetGamePaused false)))))

(fn ConstructionScript)

(fn AddMappingInput
  (bind _asplayer_controller (Utilities|Casting|CastToPlayerController (Pawn|GetController)))
  (Utilities|IsValid (PlayerController|LocalPlayerSubsystems|GetEnhancedInputLocalPlayerSubsystem _asplayer_controller)
    (:Is%20Valid
      (Input|AddMappingContext (PlayerController|LocalPlayerSubsystems|GetEnhancedInputLocalPlayerSubsystem _asplayer_controller) "/Game/BP/Input/IMC_Slime.IMC_Slime" 0 (Utilities|Struct|MakeModifyContextOptions true false)))))

(fn StretchSlime
  (bind _returnvalue (Transformation|GetActorRotation))
  (bind _stretchvector (Variables|Default|GetStretchVector))
  (bind _stretchvector_2 (Variables|Default|GetStretchVector))
  (bind (_x _y) (Math|Vector2D|BreakVector2D _stretchvector))
  (bind _returnvalue_2 (Math|Float|Absolute(Float) (.yaw _returnvalue)))
  (bind _returnvalue_3 (* (.pitch _returnvalue) -1.0))
  (bind _returnvalue_4 (Math|Float|NearlyEqual(Float) _returnvalue_2 1.8e+02 1.0))
  (bind _returnvalue_5 (Math|Float|SelectFloat _returnvalue_3 (.pitch _returnvalue) _returnvalue_4))
  (bind _returnvalue_6 (Class|KismetMathLibrary|GetRotated2D _stretchvector_2 _returnvalue_5))
  (bind (_x_2 _y_2) (Math|Vector2D|BreakVector2D _returnvalue_6))
  (Components|Box|SetBoxExtent (Variables|Default|GetBox) (+ (Variables|Default|GetBaseSize) (Math|Vector|ClampVectorSize (* (Math|Vector|VectorGetAbs (Math|Vector|Normalize (Math|Vector|MakeVector _x_2 0.0 _y_2))) (Variables|Default|GetStretchLength)) 0.0 (Variables|Default|GetStretchMaxLength))) true)
  (Transformation|SetActorLocation (+ (Variables|Default|GetStretchStartLocation) (Math|Vector|ClampVectorSize (Math|Vector|MakeVector (* _x -1.0) 0.0 _y) 0.0 (Variables|Default|GetStretchMaxLength))) true false))

(fn InitDebugWidget
  (bind _returnvalue (UserInterface|CreateWidget "/Game/BP/HUD/Debug/WBP_DebugTouch.WBP_DebugTouch_C"))
  (UserInterface|Viewport|AddtoViewport _returnvalue 0)
  (bind _output_get (Variables|Default|SetWBP_DebugTouch _returnvalue))
  (bind _output_get_2 (Variables|/Game/BP/HUD/Debug/WBP_DebugTouch.WBP_DebugTouch_C|SetTouchStart _output_get (Variables|Default|GetTouchStart)))
  (Variables|/Game/BP/HUD/Debug/WBP_DebugTouch.WBP_DebugTouch_C|SetTouchMoved _output_get _output_get_2)
  (Variables|/Game/BP/HUD/Debug/WBP_DebugTouch.WBP_DebugTouch_C|SetMaxSize _output_get (Variables|Default|GetStretchMaxLength)))

(fn UpdateDebugWidget
  (bind _wbp_debugtouch (Variables|Default|GetWBP_DebugTouch))
  (Variables|/Game/BP/HUD/Debug/WBP_DebugTouch.WBP_DebugTouch_C|SetTouchMoved _wbp_debugtouch (Variables|Default|GetTouchMoved))
  (Variables|/Game/BP/HUD/Debug/WBP_DebugTouch.WBP_DebugTouch_C|SetStretchAngle _wbp_debugtouch (Variables|Default|GetStretchAngle)))

(fn RemoveDebugWidget
  (bind _wbp_debugtouch (Variables|Default|GetWBP_DebugTouch))
  (Utilities|IsValid _wbp_debugtouch
    (:Is%20Valid
      (Widget|RemovefromParent _wbp_debugtouch))))

(fn CalculateStretchParameters
  (params (TouchEnd :type Vector%202D%20Structure))
  (Variables|Default|SetStretchVector (- (Variables|Default|GetTouchStart) TouchEnd))
  (Variables|Default|SetStretchLength (Math|Float|Clamp(Float) (Math|Vector2D|Vector2DLength (Variables|Default|GetStretchVector)) 0.0 (Variables|Default|GetStretchMaxLength)))
  (Variables|Default|SetStretchAngle (* (Class|KismetMathLibrary|DegAcos (Math|Vector2D|DotProduct(2D) (Math|Vector2D|Normalize2D (Variables|Default|GetStretchVector)) "(X=0.000000,Y=1.000000)")) (Math|Float|Sign(Float) (Class|KismetMathLibrary|CrossProduct2D (Math|Vector2D|Normalize2D (Variables|Default|GetStretchVector)) "(X=0.000000,Y=1.000000)")) -1.0)))

(fn StretchImpulse
  (bind _stretchangle (Variables|Default|GetStretchAngle))
  (bind _stretchvector (Variables|Default|GetStretchVector))
  (bind (_x _y) (Math|Vector2D|BreakVector2D _stretchvector))
  (Physics|SetSimulatePhysics (Variables|Default|GetBox) false)
  (Class|PrimitiveComponent|SetAngularDamping (Variables|Default|GetBox) 0.1)
  (Physics|SetSimulatePhysics (Variables|Default|GetBox) true)
  (Physics|AddImpulse (Variables|Default|GetBox) (* (Math|Vector|Normalize (Math|Vector|MakeVector (* _x -1.0) 0.0 _y)) (* (Variables|Default|GetStretchLength) (Variables|Default|GetStretchImpulseStrength))) "None" true)
  (if (<= (Math|Float|Absolute(Float) _stretchangle) 65.0)
    (Class|PrimitiveComponent|AddAngularImpulseinDegrees (Variables|Default|GetBox) (Math|Vector|MakeVector 0.0 (* (Math|Float|Sign(Float) _stretchangle) (Variables|Default|GetStretchLength) 2.0) 0.0) "None" true)))

(fn FakeGravity
  (if (Physics|IsSimulatingPhysics (Variables|Default|GetBox) "None")
    (Physics|AddForce (Variables|Default|GetBox) "0.000000,0.000000,-5000.000000" "None" true)))

(fn RemoveMappingInput
  (bind _asplayer_controller (Utilities|Casting|CastToPlayerController (Pawn|GetController)))
  (Utilities|IsValid (PlayerController|LocalPlayerSubsystems|GetEnhancedInputLocalPlayerSubsystem _asplayer_controller)
    (:Is%20Valid
      (Input|RemoveMappingContext (PlayerController|LocalPlayerSubsystems|GetEnhancedInputLocalPlayerSubsystem _asplayer_controller) "/Game/BP/Input/IMC_Slime.IMC_Slime" (Utilities|Struct|MakeModifyContextOptions false true))
      (CallFunction|RemoveDebugWidget)
      (CallFunction|StartShrinking))))

(fn UpdateSize
  (params (Amount :type Float%20%28double-precision%29))
  (Variables|Default|SetStretchMaxLength (Math|Float|Max(Float) (+ (Variables|Default|GetStretchMaxLength) Amount) 1e+02))
  (Variables|Default|SetBaseSize (Math|Vector|SelectVector "50.000000,50.000000,50.000000" (+ (Variables|Default|GetBaseSize) (Math|Vector|MakeVector Amount 0.0 Amount)) (<= (.X (Math|Vector|BreakVector (+ (Variables|Default|GetBaseSize) (Math|Vector|MakeVector Amount 0.0 Amount)))) 5e+01)))
  (CallFunction|StartShrinking)
  (if (and (< Amount 0.0) (> (Variables|Default|GetStretchMaxLength) 1e+02))
    (Game|SpawnActorfromClass "/Game/BP/PickUps/BP_SlimeDrop.BP_SlimeDrop_C" (Math|Transform|MakeTransform (* (+ (Transformation|GetActorLocation) (Math|Vector|MakeVector 0.0 0.0 (.SphereRadius (Collision|GetComponentBounds (Variables|Default|GetBox))))) "1.000000,0.000000,1.000000") "0, 0, 0" "1.000000,1.000000,1.000000") "AlwaysSpawn" "MultiplyWithRoot" 0 0)))