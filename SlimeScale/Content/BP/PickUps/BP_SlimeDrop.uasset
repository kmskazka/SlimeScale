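; BP_SlimeDrop is a physics-driven slime drop that turns into a BP_PickUp_Slime once it lands or touches the slime pawn.
; On BeginPlay its Box launches upward with random X drift and spin, while Tick applies strong downward acceleration.
; A hit from BP_SlimePawn, or any hit at near-zero speed, spawns the pickup above the impact on the Y=0 plane and destroys the drop.
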(event OnComponentHit(Box)
  (params (HitComponent :type Primitive%20Component%20Object%20Reference) (OtherActor :type Actor%20Object%20Reference) (OtherComp :type Primitive%20Component%20Object%20Reference) (NormalImpulse :type Vector :default "0, 0, 0") (Hit :type Hit%20Result%20Structure%20%28by%20ref%29))
  (Utilities|Casting|CastToBP_SlimePawn OtherActor
    (:then
      (Game|SpawnActorfromClass "/Game/BP/PickUps/BP_PickUp_Slime.BP_PickUp_Slime_C" (Math|Transform|MakeTransform (* (+ (.Location (Collision|BreakHitResult Hit)) "0.000000,0.000000,60.000000") "1.000000,0.000000,1.000000") "0, 0, 0" "1.000000,1.000000,1.000000") "Undefined" "MultiplyWithRoot" 0 2e+01 0 :!label _label)
      (Actor|DestroyActor))
    (:CastFailed
      (if (<= (Math|Vector|VectorLength (Transformation|GetVelocity)) 25.0)
        (goto _label)))))

(event EventBeginPlay
  (bind _box (Variables|Default|GetBox))
  (Physics|AddImpulse _box (* (Math|Vector|MakeVector (Math|Random|RandomFloatinRange -0.25 0.25) 0.0 1.0) 2e+03) "None" true)
  (Class|PrimitiveComponent|AddTorqueinDegrees _box "1000.000000,0.000000,0.000000" "None" true))

(event EventTick
  (params (DeltaSeconds :type Float%20%28single-precision%29))
  (Physics|AddForce (Variables|Default|GetBox) "0.000000,0.000000,-5000.000000" "None" true))

(fn ConstructionScript)