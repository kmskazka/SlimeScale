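; BP_PickUp_Slime is a pickup that grows the slime pawn when collected.
; It overrides OnPickup to call UpdateSize on SlimePawn with GrowAmount, while Tick and BeginPlay call the parent logic.
; BeginPlay also sets the PickUpAnim timeline to half speed.
; That timeline's update lerps the SMPickUp component vertically for a bobbing motion, though nothing in this graph starts it.
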(event EventBeginPlay
  (|CallParentFunction)
  (Components|Timeline|SetPlayRate (Variables|Default|GetPickUpAnim) 0.5))

(event Collision|EventActorBeginOverlap
  (params (OtherActor :type Actor%20Object%20Reference))
  (|CallParentFunction OtherActor) ; This node is disabled and will not be called.\nDrag off pins to build functionality.
)

(event EventTick
  (params (DeltaSeconds :type Float%20%28single-precision%29))
  (|CallParentFunction DeltaSeconds))

(event EventOnPickup
  (Default|UpdateSize (Variables|Default|GetSlimePawn) (Variables|Default|GetGrowAmount)))

(fn ConstructionScript
  (|CallParentFunction))