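; Base pickup actor that the slime pawn collects by touching it, with an empty OnPickup event as the hook for child pickups.
; The construction script gives the mesh a random yaw, and Tick rotates it by a fixed step each frame, not scaled by delta time.
; When PickUp_Box overlaps a BP_SlimePawn, it stores the pawn reference, calls OnPickup, then destroys itself.
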(event OnComponentBeginOverlap(PickUp_Box)
  (params (OverlappedComponent :type Primitive%20Component%20Object%20Reference) (OtherActor :type Actor%20Object%20Reference) (OtherComp :type Primitive%20Component%20Object%20Reference) (OtherBodyIndex :type Integer) (bFromSweep :type Boolean) (SweepResult :type Hit%20Result%20Structure%20%28by%20ref%29))
  (bind _asbp_slime_pawn (Utilities|Casting|CastToBP_SlimePawn OtherActor))
  (Variables|Default|SetSlimePawn _asbp_slime_pawn)
  (Utilities|FlowControl|Sequence
    (:then_0
      (CallFunction|OnPickup))
    (:then_1
      (Actor|DestroyActor))))

(event Custom|OnPickup)

(event EventBeginPlay)

(event Collision|EventActorBeginOverlap
  (params (OtherActor :type Actor%20Object%20Reference)))

(event EventTick
  (params (DeltaSeconds :type Float%20%28single-precision%29))
  (Transformation|AddRelativeRotation (Variables|Default|GetSM_PickUp) (Variables|Default|GetDeltaRotation) false false))

(fn ConstructionScript
  (Transformation|SetRelativeRotation (Variables|Default|GetSM_PickUp) (Math|Rotator|MakeRotator 0.0 0.0 (Math|Random|RandomFloatinRange 0.0 3.6e+02)) false false))