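; Spinning spike obstacle that knocks physics bodies away along X and shrinks the slime pawn on hit, with a brief damage cooldown.
; Tick rotates the mesh, while a timeline, with rate and start time set at BeginPlay from speed and start location, holds the lerp between PointA and PointB.
; The construction script places the mesh at the chosen endpoint; its floor material scaling is unconnected.
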(event OnComponentHit(StaticMesh)
  (params (HitComponent :type Primitive%20Component%20Object%20Reference) (OtherActor :type Actor%20Object%20Reference) (OtherComp :type Primitive%20Component%20Object%20Reference) (NormalImpulse :type Vector :default "0, 0, 0") (Hit :type Hit%20Result%20Structure%20%28by%20ref%29))
  (if (Physics|IsSimulatingPhysics OtherComp "None")
    (Physics|AddImpulse OtherComp (* (Math|Vector|MakeVector (Math|Float|Sign(Float) (.x (- (Transformation|GetActorLocation OtherActor) (Transformation|GetActorLocation)))) 0.0 0.1) 5e+02) "None" true)
    (bind _asbp_slime_pawn (Utilities|Casting|CastToBP_SlimePawn OtherActor))
    (Utilities|FlowControl|DoOnce false :!label _label
      (:Completed
        (Default|UpdateSize _asbp_slime_pawn (* (Variables|Default|GetDamageAmount) -1.0))
        (Utilities|FlowControl|Delay 0.2)
        (goto _label Reset)))))

(event EventBeginPlay
  (|CallParentFunction)
  (Components|Timeline|SetPlayRate (Variables|Default|GetTL_Movement) (/ 1.0 (Variables|Default|GetMovementSpeed)))
  (Components|Timeline|SetNewTime (Variables|Default|GetTL_Movement) (Utilities|Select :Index (Variables|Default|GetStartLocation) :NewEnumerator0 0.25 :NewEnumerator1 0.0 :NewEnumerator2 0.5)))

(event Collision|EventActorBeginOverlap
  (params (OtherActor :type Actor%20Object%20Reference))
  (|CallParentFunction OtherActor) ; This node is disabled and will not be called.\nDrag off pins to build functionality.
)

(event EventTick
  (params (DeltaSeconds :type Float%20%28single-precision%29))
  (|CallParentFunction DeltaSeconds)
  (Transformation|AddRelativeRotation (Variables|Default|GetStaticMesh) (Variables|Default|GetDeltaRotation) false false))

(fn ConstructionScript
  (|CallParentFunction)
  (switch Utilities|FlowControl|Switch|SwitchonE_StartLocation (Variables|Default|GetStartLocation)
    (:NewEnumerator1
      (Transformation|SetRelativeLocation (Variables|Default|GetStaticMesh) (Variables|Default|GetPointA) false false))
    (:NewEnumerator2
      (Transformation|SetRelativeLocation (Variables|Default|GetStaticMesh) (Variables|Default|GetPointB) false false))))